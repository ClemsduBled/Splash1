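; Hero_BP is the player character, with camera-relative movement, look, jump and a punch attack.
; Jump, landing and punch set flags on LutinAnimationBP to drive animations.
; Punch calls Hit, a forward line trace from below the actor's center that calls Die on any Enemy_BP it strikes.
; GameOver runs once, ragdolls the mesh, disables input and shows the GameOver widget with UI-only input.
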(event Custom|GameOver
  (bind _returnvalue (Game|GetPlayerController 0))
  ;[1 1 1] Game Over
  (Utilities|FlowControl|DoOnce false
    (:Completed
      (Development|PrintString "Vous êtes mort")
      (Physics|SetSimulatePhysics (Variables|Character|GetMesh) true)
      (Input|DisableInput (Game|GetPlayerController 0))
      (bind _returnvalue_2 (UserInterface|CreateWidget "/Game/Self_Loathing/Widgets/GameOver.GameOver_C"))
      (UserInterface|Viewport|AddtoViewport _returnvalue_2 0)
      (Variables|/Script/Engine.PlayerController|SetbShowMouseCursor _returnvalue true)
      (Input|SetInputModeUIOnly _returnvalue _returnvalue_2 "DoNotLock"))))

(event EventOnLanded
  (params (Hit :type Hit%20Result%20Structure%20%28by%20ref%29))
  (bind _aslutin_animation_bp (Utilities|Casting|CastToLutinAnimationBP (Components|SkeletalMesh|GetAnimInstance (Variables|Character|GetMesh))))
  (Variables|/Game/Self_Loathing/Hero/Animation/LutinAnimationBP.LutinAnimationBP_C|SetJump? _aslutin_animation_bp false))

(event Input|ActionEvents|InputActionJump
  (params (Key :type Key%20Structure))
  (:Pressed
    (Character|Jump)
    (bind _aslutin_animation_bp (Utilities|Casting|CastToLutinAnimationBP (Components|SkeletalMesh|GetAnimInstance (Variables|Character|GetMesh))))
    (Variables|/Game/Self_Loathing/Hero/Animation/LutinAnimationBP.LutinAnimationBP_C|SetJump? _aslutin_animation_bp true)))

(event Input|ActionEvents|InputActionPunch
  (params (Key :type Key%20Structure))
  (:Pressed
    (CallFunction|Hit)
    (bind _aslutin_animation_bp (Utilities|Casting|CastToLutinAnimationBP (Components|SkeletalMesh|GetAnimInstance (Variables|Character|GetMesh))))
    (Variables|/Game/Self_Loathing/Hero/Animation/LutinAnimationBP.LutinAnimationBP_C|SetAttack _aslutin_animation_bp true)
    (Utilities|FlowControl|Delay 0.5)
    (Variables|/Game/Self_Loathing/Hero/Animation/LutinAnimationBP.LutinAnimationBP_C|SetAttack _aslutin_animation_bp false)))

(event Input|AxisEvents|InputAxisMoveForward
  (params (AxisValue :type Float%20%28single-precision%29))
  ;[1 1 1] Déplacement du personnage
  (Pawn|Input|AddMovementInput (Math|Vector|GetForwardVector (Variables|Default|GetCamera)) AxisValue false))

(event Input|AxisEvents|InputAxisTurn
  (params (AxisValue :type Float%20%28single-precision%29))
  ;[1 1 1] Orientation of the camera
  (Pawn|Input|AddControllerYawInput AxisValue))

(event Input|AxisEvents|InputAxisLookUp
  (params (AxisValue :type Float%20%28single-precision%29))
  ;[1 1 1] Orientation of the camera
  (Pawn|Input|AddControllerPitchInput AxisValue))

(event Input|AxisEvents|InputAxisMoveRight
  (params (AxisValue :type Float%20%28single-precision%29))
  ;[1 1 1] Déplacement du personnage
  (Pawn|Input|AddMovementInput (Math|Vector|GetRightVector (Variables|Default|GetCamera)) AxisValue false))

(fn ConstructionScript)

(fn Hit
  (bind _returnvalue (Transformation|GetActorLocation))
  (bind _returnvalue_2 (- _returnvalue "0, 0,50.000000"))
  (bind (_outhit _returnvalue_3) (Collision|LineTraceByChannel _returnvalue_2 (+ _returnvalue_2 (* (Math|Vector|GetForwardVector (Variables|Collision|GetCapsuleComponent)) (Variables|Default|GetPunchDistance))) "TraceTypeQuery1" false 0 "ForDuration"))
  (if _returnvalue_3
    (bind _asenemy_bp (Utilities|Casting|CastToEnemy_BP (.HitActor (Collision|BreakHitResult _outhit))))
    (Default|Die _asenemy_bp)))